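; Player-controllable tank Blueprint that wires its components into native-style setup calls and maps input to aiming, driving and firing.
; BeginPlay passes the barrel and turret to SetTankReference and both tracks to the TankMovement component.
; Aim axes rotate the azimuth gimbal and spring arm, scaled by delta time for frame-rate independence.
; Move and turn axes send intents to TankMovement and Fire calls the fire function, while per-track throttle events are empty.
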(event `self.ReceiveBeginPlay`
  (`self.SetTankReference` (`self.TankBarrel`) (`self.TankTurret`))
  (`TankMovementComponent.Initialise` (`self.TankMovement`) (`self.TankTrack_L`) (`self.TankTrack_R`)))

(event `InputAxis|AimAizmuth`
  (params (AxisValue :type "Float (single-precision)"))
  ;[1 1 1] Camera Control binding control the tank aim aizmuth and elevation
  (`SceneComponent.K2_AddLocalRotation` (`self.AzimuthGimbal`) (`KismetMathLibrary.MakeRotator` 0.0 0.0 (* AxisValue (`GameplayStatics.GetWorldDeltaSeconds`) 100.0)) false false))

(event `InputAxis|Left Track Throttle`
  (params (AxisValue :type "Float (single-precision)"))
  ;[1 1 1] Input binding to C++ class
)

(event `InputAxis|Aimelevation`
  (params (AxisValue :type "Float (single-precision)"))
  ;[1 1 1] Camera Control binding control the tank aim aizmuth and elevation
  (`SceneComponent.K2_AddLocalRotation` (`self.SpringArm`) (`KismetMathLibrary.MakeRotator` 0.0 (* AxisValue (`GameplayStatics.GetWorldDeltaSeconds`) 100.0)) false false))

(event `InputAxis|Right Track Throttle`
  (params (AxisValue :type "Float (single-precision)"))
  ;[1 1 1] Input binding to C++ class
)

(event `InputAxis|Move Forward`
  (params (AxisValue :type "Float (single-precision)"))
  ;[1 1 1] Input binding to C++ class
  (`TankMovementComponent.IntendMoveForward` (`self.TankMovement`) AxisValue))

(event `InputAction|Fire`
  (params (Key :type "Key Structure"))
  ;[1 1 1] Camera Control binding control the tank aim aizmuth and elevation
  (:`Pressed`
    (`self.Fire`)))

(event `InputAxis|Turn Right`
  (params (AxisValue :type "Float (single-precision)"))
  ;[1 1 1] Input binding to C++ class
  (`TankMovementComponent.IntendTurnRight` (`self.TankMovement`) AxisValue))

(fn `UserConstructionScript`)